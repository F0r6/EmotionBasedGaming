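; Face-tracking display actor that shows a video feed on a plane and the last detected emotion as a coloured box.
; BeginPlay creates dynamic material instances for the plane and emotion box.
; Tick pushes VideoTexture into the video material and maps LastDetectedEmotion, which is not set in this graph, to the box colour.
; The Angry branch is not wired to the colour update, so its red never applies.
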(event `self.ReceiveBeginPlay`
  (bind _returnvalue (`KismetMaterialLibrary.CreateDynamicMaterialInstance` "/Game/EmotionBasedGaming/Materials/M_VideoDisplay.M_VideoDisplay"))
  (bind _output_get (set `self.VidTexture` _returnvalue))
  (`PrimitiveComponent.SetMaterial` (`self.Plane`) 0 _output_get)
  (bind _returnvalue_2 (`KismetMaterialLibrary.CreateDynamicMaterialInstance` "/Game/EmotionBasedGaming/Materials/M_EmotionBox.M_EmotionBox"))
  (bind _output_get_2 (set `self.BoxColour` _returnvalue_2))
  (`PrimitiveComponent.SetMaterial` (`self.EmotionBox`) 0 _output_get_2))

(event `self.ReceiveTick`
  (params (DeltaSeconds :type "Float (single-precision)"))
  (`MaterialInstanceDynamic.SetTextureParameterValue` (`self.VidTexture`) "VideoTexture" (`self.VideoTexture`))
  (switch `EFacialEmotion` (`self.LastDetectedEmotion`)
    (:`Neutral`
      (set `self.Value` (struct :`R` 0.28125 :`G` 0.28125 :`B` 0.28125 :`A` 1.0))
      (`MaterialInstanceDynamic.SetVectorParameterValue` (`self.BoxColour`) "ColourBox" (`self.Value`) :!label _label))
    (:`Happy`
      (set `self.Value` (struct :`R` 0.399156 :`G` 1.0 :`B` 0.0997 :`A` 1.0))
      (goto _label))
    (:`Sad`
      (set `self.Value` (struct :`G` 0.042615 :`B` 1.0 :`A` 1.0))
      (goto _label))
    (:`Angry`
      (set `self.Value` (struct :`R` 1.0 :`G` 0.060762 :`B` 0.052368 :`A` 1.0)))
    (:`Surprised`
      (set `self.Value` (struct :`R` 0.171881 :`G` 1.0 :`B` 0.899943 :`A` 1.0))
      (goto _label))
    (:`Fearful`
      (set `self.Value` (struct :`R` 0.740976 :`G` 0.149225 :`B` 1.0 :`A` 1.0))
      (goto _label))
    (:`Disgusted`
      (set `self.Value` (struct :`R` 0.160332 :`G` 0.421875 :`A` 1.0))
      (goto _label))))

(fn `UserConstructionScript`)